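; Abstract base actor for solvable elements that can be chained, each tracking a solved state and broadcasting changes through an event dispatcher.
; On BeginPlay it subscribes to the dispatchers of the Solvables keyed in its conditions map, storing each reported state.
; It becomes solved when all conditions are true, unsolved when any fails, propagating the result to listeners.
; With no conditions, UpdateSolveState simply toggles its state.
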(event Custom|SetConditionBySolvable
  (params (SolvableUpdated :type B%20Pabs%20GEN%20Solvable%20Object%20Reference) (isSolved :type Boolean))
  (Development|PrintString (Utilities|String|Append "Solvable " (Utilities|GetDisplayName SolvableUpdated) " was update and its condition will be set to " (Utilities|String|ToString(Boolean) isSolved)))
  (Utilities|Map|Add (Variables|Var|GetSolvableConditions) SolvableUpdated isSolved) ; Apprently also equivalent to "Update" (if the key is already here, it will update its corresponding value).\nOk Unreal, why not ig :}
  (StateHandlers|CheckCondsandUpdateState))

(event EventBeginPlay
  ;[0.15 0.15 0.15 0.5] Preemptive check on the amount of conditions.
  ; If there are none, stops immediately.
  (if (not (== (Utilities|Map|Length (Variables|Var|GetSolvableConditions)) 0))
    (bind _keypin (Utilities|Map|ForEachLoop(Map) (Variables|Var|GetSolvableConditions))
      (:then
        (if (Utilities|IsValid _keypin)
          (EventDispatchers|BindEventtoEDonSolveStateUpd _keypin (delegate Custom|SetConditionBySolvable))
          (Development|PrintString (Utilities|String|Append "Just subscribed to " (Utilities|GetDisplayName _keypin)) true true "(R=0.000000,G=0.660000,B=1.000000,A=1.000000)" 7.0)
          (else
            (Development|PrintString "An actor was INVALD and its condition will be ignored !" true true "(R=1.000000,G=0.000000,B=0.000000,A=1.000000)" 5.0)))))))

(event Collision|EventActorBeginOverlap
  (params (OtherActor :type Actor%20Object%20Reference)))

(event EventTick
  (params (DeltaSeconds :type Float%20%28single-precision%29)))

(event EventUpdateSolveState
  ;[0.15 0.15 0.15 0.5] Preemptive check on the amount of conditions.
  ; If there are none, act as a much simpler Solvable.
  (if (== (Utilities|Map|Length (Variables|Var|GetSolvableConditions)) 0)
    ;[0.15 0.15 0.15 0.5] Empty condition list scenario : Act like it has no restriction and flip its state.
    (StateHandlers|SetIsSolvedandNotify (not (Variables|Var|GetisSolved)))
    (else
      ;[0.15 0.15 0.15 0.5] Not empty condition list scenario : Check them all and notify if needed.
      (StateHandlers|CheckCondsandUpdateState))))

(fn ConstructionScript)

(fn SetIsSolvedandNotify
  (params (newState :type Boolean))
  (bind _self self)
  (bind _output_get (Variables|Var|SetisSolved newState))
  (Default|CallEDonSolveStateUpd _self _output_get)
  (Development|PrintString (Utilities|String|Append "Actor " (Utilities|GetDisplayName _self) " just called ED with " (Utilities|String|ToString(Boolean) _output_get)) true true "(R=0.000000,G=0.660000,B=1.000000,A=1.000000)" 4.0))

(fn CheckCondsandUpdateState
  (LocalVariables|SetareAllCondsTrue true) ; Assumption made at the start, corrected if any cond is False.
  (bind _valuepin (Utilities|Map|ForEachLoop(Map) (Variables|Var|GetSolvableConditions) :!label _label)
    (:then
      (if (not _valuepin) ; If any condition is False, break out of the loop and handle the unsolved state.\nNo need to do anything if any or all of them are True.
        ;[0.15 0.15 0.15 0.5] Case in which a condition was false : Dispatch (if relevant) and update the state. Also break out of the loop.
        (LocalVariables|SetareAllCondsTrue false) ; Corrects the starting assumption.
        (if (Variables|Var|GetisSolved) ; If previously solved, Set and Notify
          (StateHandlers|SetIsSolvedandNotify false)
          (goto _label BreakPin)
          (else
            (goto _label BreakPin)))))
    (:CompletedPin
      ;[0.15 0.15 0.15 0.5] End of the loop : If relevant, call dispatch and update the state.
      (if (LocalVariables|GetareAllCondsTrue) ; Once the loop ends, check the assumption of the beginning.\nIf it still holds, notify.
        (StateHandlers|SetIsSolvedandNotify true)))))