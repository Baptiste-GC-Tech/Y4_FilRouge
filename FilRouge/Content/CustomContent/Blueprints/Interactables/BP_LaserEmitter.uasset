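; Interactable laser emitter that, when a player interacts, fires a ray from a local offset along its forward vector and bounces it off blocking surfaces.
; DoOneRaycast calls OnLightSolve on overlapped BPI_SolvableByLight actors via multi-trace, then line-traces for the blocking hit.
; PrepareNextRaycast mirrors the direction around the normal from a slightly offset impact point, looping until a miss or the bounce cap.
; The beam appears only as timed debug lines.
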(event EventBeginPlay
  (|CallParentFunction))

(event EventTick
  (params (DeltaSeconds :type Float%20%28single-precision%29))
  (|CallParentFunction DeltaSeconds))

(event EventOnPlayerInteract
  (params (InteractingPlayerController :type Player%20Controller%20Object%20Reference))
  (bind _returnvalue (Transformation|GetActorLocation))
  (bind _returnvalue_2 (Transformation|GetActorTransform))
  (bind _initialraycastlocaloffset (Variables|Var|Raycasting|GetInitialRaycastLocalOffset))
  (bind _returnvalue_3 (Math|Transform|TransformDirection _returnvalue_2 _initialraycastlocaloffset))
  (bind _returnvalue_4 (+ _returnvalue _returnvalue_3))
  (|CallParentFunction InteractingPlayerController)
  (Variables|Var|Raycasting|SetSecurityCounter 0)
  ;[0.15 0.15 0.15 0.5] Prepares the first raycast
  (Variables|Var|Raycasting|SetCurRaycastStartingPoint _returnvalue_4)
  (Variables|Var|Raycasting|SetCurRaycastEndingPoint (+ _returnvalue_4 (* (Variables|Var|Raycasting|GetraycastLength) (Math|Vector|GetForwardVector (Transformation|GetActorRotation)))))
  ;[0.15 0.15 0.15 0.5] Do...
  (bind (_impactpoint _impactnormal _rayforwardvector) (CallFunction|DoOneRaycast))
  (if (Variables|Var|Raycasting|GethasLastRayHit)
    (CallFunction|PrepareNextRaycast _impactpoint _impactnormal _rayforwardvector)
    ;[0.15 0.15 0.15 0.5] ...While
    (while (and (Variables|Var|Raycasting|GethasLastRayHit) (< (Variables|Var|Raycasting|GetSecurityCounter) (Variables|Var|Raycasting|GetMaxSubsequentRaycasts)))
      (bind (_impactpoint_2 _impactnormal_2 _rayforwardvector_2) (CallFunction|DoOneRaycast))
      (CallFunction|PrepareNextRaycast _impactpoint_2 _impactnormal_2 _rayforwardvector_2)
      (Math|Integer|IncrementInt (Variables|Var|Raycasting|GetSecurityCounter)))
    (Development|PrintString (Utilities|String|Append "Subsequent rays fired : " (Utilities|String|ToString(Integer) (Variables|Var|Raycasting|GetSecurityCounter))) true true "(R=0.000000,G=0.660000,B=1.000000,A=1.000000)" (Variables|Var|Raycasting|GetDebug%20Draw%20Time))))

(fn ConstructionScript
  (|CallParentFunction))

(fn DoOneRaycast
  (Development|PrintString "Hello")
  (bind _outhits (Collision|MultiLineTraceByChannel (Variables|Var|Raycasting|GetCurRaycastStartingPoint) (Variables|Var|Raycasting|GetCurRaycastEndingPoint) "TraceTypeQuery3" false 0 "None"))
  (for _array_element _outhits
    ;[0.15 0.15 0.15 0.5] Tests if the line trace overlapped with a BPI_SolvableByLight
    (if (and (not (.bBlockingHit (Collision|BreakHitResult _array_element))) (Utilities|DoesObjectImplementInterface (.HitActor (Collision|BreakHitResult _array_element)) "/Game/CustomContent/Blueprints/Systems/SpecificSolvables/LightPuzzle/BPI_SolvableByLight.BPI_SolvableByLight_C"))
      (Default|OnLightSolve (.AsBPI%20Solvable%20by%20Light (Utilities|Casting|CastToBPI_SolvableByLight (.HitActor (Collision|BreakHitResult _array_element)))) self)))
  (bind _outhit (Collision|LineTraceByChannel (Variables|Var|Raycasting|GetCurRaycastStartingPoint) (Variables|Var|Raycasting|GetCurRaycastEndingPoint) "TraceTypeQuery3" false 0 "ForDuration" true "(R=1.000000,G=0.000000,B=0.000000,A=1.000000)" "(R=0.000000,G=1.000000,B=0.000000,A=1.000000)" (Variables|Var|Raycasting|GetDebug%20Draw%20Time)))
  (Variables|Var|Raycasting|SethasLastRayHit (.bBlockingHit (Collision|BreakHitResult _outhit)))
  (return (+ (.ImpactPoint (Collision|BreakHitResult _outhit)) (* (Math|Float|MakeLiteralFloat 0.01) (.ImpactNormal (Collision|BreakHitResult _outhit)))) (.ImpactNormal (Collision|BreakHitResult _outhit)) (Math|Vector|Normalize (- (Variables|Var|Raycasting|GetCurRaycastEndingPoint) (Variables|Var|Raycasting|GetCurRaycastStartingPoint)))))

(fn PrepareNextRaycast
  (params (LastImpactPoint :type Vector) (LastImpactNormal :type Vector) (LastRayForwardVector :type Vector))
  (Variables|Var|Raycasting|SetCurRaycastStartingPoint LastImpactPoint)
  (Variables|Var|Raycasting|SetCurRaycastEndingPoint (+ LastImpactPoint (* (Math|Vector|MirrorVectorbyNormal LastRayForwardVector LastImpactNormal) (Variables|Var|Raycasting|GetraycastLength)))))