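; BP_LightReactor is a reactor Blueprint whose point light changes color when it is interacted with.
; The OnInteractionNOARGS event drives a FlipFlop that alternates between red and green and applies the result to the PointLight component.
; BeginPlay, overlap and Tick are unused, and the construction script only calls its parent.
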(event EventBeginPlay
  (|CallParentFunction) ; This node is disabled and will not be called.\nDrag off pins to build functionality.
)

(event Collision|EventActorBeginOverlap
  (params (OtherActor :type Actor%20Object%20Reference))
  (|CallParentFunction OtherActor) ; This node is disabled and will not be called.\nDrag off pins to build functionality.
)

(event EventTick
  (params (DeltaSeconds :type Float%20%28single-precision%29))
  (|CallParentFunction DeltaSeconds) ; This node is disabled and will not be called.\nDrag off pins to build functionality.
)

(event EventOnInteractionNOARGS
  (params (InteractableCaller :type B%20Pabs%20GEN%20Interactable%20Object%20Reference))
  (Utilities|FlowControl|FlipFlop
    (:A
      (Variables|Default|SetNewLinearColor "(R=1.000000,G=0.000000,B=0.000000,A=1.000000)"))
    (:B
      (Variables|Default|SetNewLinearColor "(R=0.000000,G=1.000000,B=0.000000,A=1.000000)")))
  (Rendering|Components|Light|SetLightColor (Variables|Default|GetPointLight) (Variables|Default|GetNewLinearColor) true))

(fn ConstructionScript
  (|CallParentFunction))