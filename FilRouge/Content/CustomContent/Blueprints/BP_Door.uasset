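; BP_Door is a two-panel sliding door that toggles between open and closed.
; OpenDoor and CloseDoor snap the left and right panels apart or together along X with relative location changes, without animation, and update the IsOpen flag.
; ChangeDoorState prints a debug string and calls the opposite action based on IsOpen; nothing in this Blueprint triggers it, so it relies on external callers.
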(event Custom|OpenDoor
  ;[0.15 0.1298 0.007428 0.5] Door's panel movement
  (Utilities|FlowControl|Sequence
    (:then_0
      (Transformation|SetRelativeLocation (Variables|Default|GetRight%20Panel) "185.000000,0.000000,150.000000" false false))
    (:then_1
      (Transformation|SetRelativeLocation (Variables|Default|GetLeftPanel) "-185.000000,0.000000,150.000000" false false))
    (:then_2
      (Variables|Default|SetisOpen true))))

(event Custom|ChangeDoorState
  (Development|PrintString "Calling BP_Door's \"ChangeDoorState\"")
  (if (Variables|Default|GetisOpen)
    (CallFunction|CloseDoor)
    (else
      (CallFunction|OpenDoor))))

(event Custom|CloseDoor
  ;[0.15 0.1298 0.007428 0.5] Door's panel movement
  (Utilities|FlowControl|Sequence
    (:then_0
      (Transformation|SetRelativeLocation (Variables|Default|GetRight%20Panel) "85.000000,0.000000,150.000000" false false))
    (:then_1
      (Transformation|SetRelativeLocation (Variables|Default|GetLeftPanel) "-85.000000,0.000000,150.000000" false false))
    (:then_2
      (Variables|Default|SetisOpen false))))

(event EventBeginPlay)

(event Collision|EventActorBeginOverlap
  (params (OtherActor :type Actor%20Object%20Reference)))

(event EventTick
  (params (DeltaSeconds :type Float%20%28single-precision%29)))

(fn ConstructionScript)