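; BP_LightReceiver is a solvable puzzle object that represents a sensor for light from laser emitters.
; It leaves solve-state logic to its parent and binds to the solve-state-updated dispatcher on BeginPlay.
; That feedback handler swaps the SensorPlate material between on and off variants.
; OnLightSolve only prints a debug message naming the emitter, without changing the solve state itself.
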(event Custom|OnSolveStateUpdFeedback
  (params (SolvableUpdated :type B%20Pabs%20GEN%20Solvable%20Object%20Reference) (isSolved :type Boolean))
  (bind _sensorplate (Variables|Default|GetSensorPlate))
  (if isSolved
    (Rendering|Material|SetMaterial _sensorplate 0 "/Game/CustomContent/Materials/LightPuzzle/MI_LightReceiverSurfaceOn.MI_LightReceiverSurfaceOn")
    (else
      (Rendering|Material|SetMaterial _sensorplate 0 "/Game/CustomContent/Materials/LightPuzzle/MI_LightReceiverSurfaceOff.MI_LightReceiverSurfaceOff"))))

(event EventBeginPlay
  (|CallParentFunction)
  (EventDispatchers|BindEventtoEDonSolveStateUpd (delegate Custom|OnSolveStateUpdFeedback)) ; Subscription of the Player Feedback
)

(event EventOnLightSolve
  (params (LaserEmitter :type BP%20Laser%20Emitter%20Object%20Reference))
  (Development|PrintString (Utilities|String|Append "Solve By Light attempt received from " (Utilities|GetDisplayName LaserEmitter)) true true "(R=0.370821,G=0.041667,B=1.000000,A=1.000000)" 1e+01))

(event EventTick
  (params (DeltaSeconds :type Float%20%28single-precision%29))
  (|CallParentFunction DeltaSeconds) ; This node is disabled and will not be called.\nDrag off pins to build functionality.
)

(event EventUpdateSolveState
  ;[0.15 0.15 0.15 0.5] No need for extra logic
  (|CallParentFunction))

(fn ConstructionScript
  (|CallParentFunction))